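; Water plane actor that renders a selectable liquid preset (water, dirty, toxic, oil or magic) with a Gerstner wave material.
; Construction script and BeginPlay each create a dynamic material instance on the mesh, then ApplyLiquidPreset sets its color, opacity, wave and foam parameters.
; Viscosity is stored per preset but not sent to the material.
; AddWaterImpact drives one material ripple from location, strength and game time, so each impact overwrites the last.
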(event `self.ReceiveBeginPlay`
  (bind _returnvalue (`KismetMaterialLibrary.CreateDynamicMaterialInstance` "/LiquidFX/Materials/Masters/Water/M_WaterMaster_Gerstner.M_WaterMaster_Gerstner"))
  (bind _output_get (set `self.WaterMID` _returnvalue))
  (`PrimitiveComponent.SetMaterial` (`self.StaticMesh`) 0 _output_get)
  (`self.ApplyLiquidPreset` (`self.LiquidType`))
  (`parent.ReceiveBeginPlay`))

(fn `AddWaterImpact`
  (params (ImpactLocation :type "Vector Structure") (ImpactStrength :type "Float (double-precision)"))
  (bind _watermid (`self.WaterMID`))
  (`/Engine/EditorBlueprintResources/StandardMacros.IsValid` _watermid
    (:`Is Valid`
      (`MaterialInstanceDynamic.SetVectorParameterValue` _watermid "RippleCenter" (`KismetMathLibrary.Conv_VectorToLinearColor` ImpactLocation))
      (`MaterialInstanceDynamic.SetScalarParameterValue` _watermid "RippleStartTime" (`KismetSystemLibrary.GetGameTimeInSeconds`))
      (`MaterialInstanceDynamic.SetScalarParameterValue` _watermid "RippleStrength" ImpactStrength))
    (:`Is Not Valid`
      (`KismetSystemLibrary.PrintString` "BP_EaterPlane_material not valid"))))

(fn `ApplyLiquidPreset`
  (params (LiquidType :type "/LiquidFX/Blueprints/Types/E_LiquidType Enum" :default "NewEnumerator0"))
  (bind _watermid (`self.WaterMID`))
  (bind _watermid_2 (`self.WaterMID`))
  (bind _watermid_3 (`self.WaterMID`))
  (bind _watermid_4 (`self.WaterMID`))
  (bind _watermid_5 (`self.WaterMID`))
  (switch `/LiquidFX/Blueprints/Types/E_LiquidType` LiquidType
    (:`NewEnumerator0`
      ; Water
      (set `self.Viscosity` 1.0)
      (bind _output_get (set `self.WaveAmplitude` 20.0))
      (bind _output_get_2 (set `self.WaveSpeed` 1.0))
      (bind _output_get_3 (set `self.FoamIntensity` 1.0))
      (bind _output_get_4 (set `self.Opacity` 0.6))
      (bind _output_get_5 (set `self.ShoreFoamIntensity` 2.0))
      (`MaterialInstanceDynamic.SetVectorParameterValue` _watermid "BaseColor" (struct :`R` 0.144128 :`G` 0.258183 :`B` 0.863157 :`A` 1.0))
      (`MaterialInstanceDynamic.SetVectorParameterValue` _watermid "DepthColor" (struct :`G` 0.138432 :`B` 0.323143 :`A` 1.0))
      (`MaterialInstanceDynamic.SetScalarParameterValue` _watermid "Opacity" _output_get_4)
      (`MaterialInstanceDynamic.SetScalarParameterValue` _watermid "FoamIntensity" _output_get_3)
      (`MaterialInstanceDynamic.SetScalarParameterValue` _watermid "Speed" _output_get_2)
      (`MaterialInstanceDynamic.SetScalarParameterValue` _watermid "Amplitude" _output_get)
      (`MaterialInstanceDynamic.SetScalarParameterValue` _watermid "ShoreFoamIntensity" _output_get_5))
    (:`NewEnumerator1`
      ; Dirty Liquid
      (set `self.Viscosity` 2.5)
      (bind _output_get_6 (set `self.WaveAmplitude` 12.0))
      (bind _output_get_7 (set `self.WaveSpeed` 0.5))
      (bind _output_get_8 (set `self.FoamIntensity` 0.2))
      (bind _output_get_9 (set `self.Opacity` 0.95))
      (bind _output_get_10 (set `self.ShoreFoamIntensity` 2.0))
      (`MaterialInstanceDynamic.SetVectorParameterValue` _watermid_4 "BaseColor" (struct :`R` 0.056128 :`G` 0.066626 :`B` 0.082283 :`A` 1.0))
      (`MaterialInstanceDynamic.SetVectorParameterValue` _watermid_4 "DepthColor" (struct :`R` 0.0185 :`G` 0.03434 :`B` 0.114435 :`A` 1.0))
      (`MaterialInstanceDynamic.SetScalarParameterValue` _watermid_4 "Opacity" _output_get_9)
      (`MaterialInstanceDynamic.SetScalarParameterValue` _watermid_4 "FoamIntensity" _output_get_8)
      (`MaterialInstanceDynamic.SetScalarParameterValue` _watermid_4 "Speed" _output_get_7)
      (`MaterialInstanceDynamic.SetScalarParameterValue` _watermid_4 "Amplitude" _output_get_6)
      (`MaterialInstanceDynamic.SetScalarParameterValue` _watermid_4 "ShoreFoamIntensity" _output_get_10)
      (`MaterialInstanceDynamic.SetVectorParameterValue` _watermid_4 "FoamColor" (struct :`R` 0.027262 :`G` 0.006042 :`B` 0.177083 :`A` 1.0)))
    (:`NewEnumerator2`
      ; ToxicLiquid
      (set `self.Viscosity` 1.5)
      (bind _output_get_11 (set `self.WaveAmplitude` 15.0))
      (bind _output_get_12 (set `self.WaveSpeed` 0.8))
      (bind _output_get_13 (set `self.FoamIntensity` 0.1))
      (bind _output_get_14 (set `self.Opacity` 1.0))
      (bind _output_get_15 (set `self.ShoreFoamIntensity` 0.0))
      (`MaterialInstanceDynamic.SetVectorParameterValue` _watermid_5 "BaseColor" (struct :`G` 0.25 :`B` 0.024353 :`A` 1.0))
      (`MaterialInstanceDynamic.SetVectorParameterValue` _watermid_5 "DepthColor" (struct :`R` 0.000146 :`G` 0.1875 :`B` 0.019082 :`A` 1.0))
      (`MaterialInstanceDynamic.SetScalarParameterValue` _watermid_5 "Opacity" _output_get_14)
      (`MaterialInstanceDynamic.SetScalarParameterValue` _watermid_5 "FoamIntensity" _output_get_13)
      (`MaterialInstanceDynamic.SetScalarParameterValue` _watermid_5 "Speed" _output_get_12)
      (`MaterialInstanceDynamic.SetScalarParameterValue` _watermid_5 "Amplitude" _output_get_11)
      (`MaterialInstanceDynamic.SetScalarParameterValue` _watermid_5 "ShoreFoamIntensity" _output_get_15)
      (`MaterialInstanceDynamic.SetVectorParameterValue` _watermid_5 "FoamColor" (struct :`A` 1.0)))
    (:`NewEnumerator3`
      ; Oil
      (set `self.Viscosity` 5.0)
      (bind _output_get_16 (set `self.WaveAmplitude` 6.0))
      (bind _output_get_17 (set `self.WaveSpeed` 0.25))
      (bind _output_get_18 (set `self.FoamIntensity` 1.0))
      (bind _output_get_19 (set `self.Opacity` 1.0))
      (bind _output_get_20 (set `self.ShoreFoamIntensity` 2.0))
      (`MaterialInstanceDynamic.SetVectorParameterValue` _watermid_3 "BaseColor" (struct :`R` 0.093059 :`G` 0.036889 :`B` 0.000304 :`A` 1.0))
      (`MaterialInstanceDynamic.SetVectorParameterValue` _watermid_3 "DepthColor" (struct :`A` 1.0))
      (`MaterialInstanceDynamic.SetScalarParameterValue` _watermid_3 "Opacity" _output_get_19)
      (`MaterialInstanceDynamic.SetScalarParameterValue` _watermid_3 "FoamIntensity" _output_get_18)
      (`MaterialInstanceDynamic.SetScalarParameterValue` _watermid_3 "Speed" _output_get_17)
      (`MaterialInstanceDynamic.SetScalarParameterValue` _watermid_3 "Amplitude" _output_get_16)
      (`MaterialInstanceDynamic.SetScalarParameterValue` _watermid_3 "ShoreFoamIntensity" _output_get_20)
      (`MaterialInstanceDynamic.SetVectorParameterValue` _watermid_3 "FoamColor" (struct :`A` 1.0)))
    (:`NewEnumerator4`
      ; MagicLiquid
      (set `self.Viscosity` 0.8)
      (bind _output_get_21 (set `self.WaveAmplitude` 25.0))
      (bind _output_get_22 (set `self.WaveSpeed` 1.3))
      (bind _output_get_23 (set `self.FoamIntensity` 0.6))
      (bind _output_get_24 (set `self.Opacity` 0.55))
      (bind _output_get_25 (set `self.ShoreFoamIntensity` 1.0))
      (`MaterialInstanceDynamic.SetVectorParameterValue` _watermid_2 "BaseColor" (struct :`R` 0.034465 :`G` 0.115191 :`B` 0.5 :`A` 1.0))
      (`MaterialInstanceDynamic.SetVectorParameterValue` _watermid_2 "DepthColor" (struct :`R` 0.186917 :`G` 0.009296 :`B` 0.337164 :`A` 1.0))
      (`MaterialInstanceDynamic.SetScalarParameterValue` _watermid_2 "Opacity" _output_get_24)
      (`MaterialInstanceDynamic.SetScalarParameterValue` _watermid_2 "FoamIntensity" _output_get_23)
      (`MaterialInstanceDynamic.SetScalarParameterValue` _watermid_2 "Speed" _output_get_22)
      (`MaterialInstanceDynamic.SetScalarParameterValue` _watermid_2 "Amplitude" _output_get_21)
      (`MaterialInstanceDynamic.SetScalarParameterValue` _watermid_2 "ShoreFoamIntensity" _output_get_25)
      (`MaterialInstanceDynamic.SetVectorParameterValue` _watermid_2 "FoamColor" (struct :`R` 0.882552 :`G` 0.083374 :`B` 1.0 :`A` 1.0)))))

(fn `UserConstructionScript`
  (`parent.UserConstructionScript`)
  (bind _returnvalue (`KismetMaterialLibrary.CreateDynamicMaterialInstance` "/LiquidFX/Materials/Masters/Water/M_WaterMaster_Gerstner.M_WaterMaster_Gerstner"))
  (bind _output_get (set `self.WaterMID` _returnvalue))
  (`PrimitiveComponent.SetMaterial` (`self.StaticMesh`) 0 _output_get)
  (`self.ApplyLiquidPreset` (`self.LiquidType`)))