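; Water plane actor that renders with a Gerstner-wave material and exposes height, bounds and impact-ripple functions.
; BeginPlay puts a dynamic instance of the water material on the mesh, and AddWaterImpact writes ripple center, start time and strength to it, holding one ripple at a time.
; GetWaterHeight computes a single directional cosine wave on the CPU from wave variables.
; IsPointInsideWater tests only X and Y against scaled mesh bounds plus a margin.
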(event `self.ReceiveBeginPlay`
  (bind _returnvalue (`KismetMaterialLibrary.CreateDynamicMaterialInstance` "/Game/Materials/M_WaterMaster_Gerstner.M_WaterMaster_Gerstner"))
  (bind _output_get (set `self.WaterMID` _returnvalue))
  (`PrimitiveComponent.SetMaterial` (`self.StaticMesh`) 0 _output_get))

(fn `AddWaterImpact`
  (params (ImpactLocation :type "Vector Structure") (ImpactStrength :type "Float (double-precision)"))
  (bind _watermid (`self.WaterMID`))
  (`MaterialInstanceDynamic.SetVectorParameterValue` _watermid "RippleCenter" (`KismetMathLibrary.Conv_VectorToLinearColor` ImpactLocation))
  (`MaterialInstanceDynamic.SetScalarParameterValue` _watermid "RippleStartTime" (`KismetSystemLibrary.GetGameTimeInSeconds`))
  (`MaterialInstanceDynamic.SetScalarParameterValue` _watermid "RippleStrength" ImpactStrength))

(fn `GetWaterHeight`
  (params (WorldPosition :type "Vector Structure") (Time :type "Float (double-precision)"))
  (returns (Height :type "Float (double-precision)"))
  (return (+ (.z (`self.K2_GetActorLocation`)) (* (`self.Amplitude`) (`KismetMathLibrary.Cos` (- (* (/ (`KismetMathLibrary.MultiplyByPi` 2.0) (`self.Wavelength`)) (`KismetMathLibrary.DotProduct2D` (`KismetMathLibrary.MakeVector2D` (* (.x WorldPosition) 1.0) (* (.y WorldPosition) 1.0)) (`KismetMathLibrary.Normal2D` (`KismetMathLibrary.MakeVector2D` (`self.DirX`) (`self.DirY`))))) (* Time (`self.Speed`))))))))

(fn `IsPointInsideWater`
  (params (Point :type "Vector Structure"))
  (returns (IsInside :type Boolean))
  (bind _returnvalue (`ActorComponent.GetOwner` (`self.StaticMesh`)))
  (return (and (<= (`KismetMathLibrary.Abs` (.x (`KismetMathLibrary.InverseTransformLocation` (`self.GetTransform` _returnvalue) Point))) (+ (* (.x (`self.GetActorScale3D` _returnvalue)) (.x (`.Max` (`StaticMeshComponent.GetLocalBounds` (`self.StaticMesh`))))) 50.0)) (<= (`KismetMathLibrary.Abs` (.y (`KismetMathLibrary.InverseTransformLocation` (`self.GetTransform` _returnvalue) Point))) (+ (* (.y (`self.GetActorScale3D` _returnvalue)) (.y (`.Max` (`StaticMeshComponent.GetLocalBounds` (`self.StaticMesh`))))) 50.0)))))

(fn `UserConstructionScript`)