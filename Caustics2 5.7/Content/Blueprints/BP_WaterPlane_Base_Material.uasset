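; Water plane Blueprint that shows ripples where impacts are reported on its surface.
; Construction script and BeginPlay each create a dynamic instance of the base material, store it as WaterMID and apply it to the static mesh.
; AddWaterImpact passes impact location, game-time start and strength to that material, leaving ripple animation to the shader.
; Each impact overwrites the same parameters, so only the latest ripple is stored.
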(event `self.ReceiveBeginPlay`
  (bind _returnvalue (`KismetMaterialLibrary.CreateDynamicMaterialInstance` (`self.BaseMaterial`)))
  (bind _output_get (set `self.WaterMID` _returnvalue))
  (`PrimitiveComponent.SetMaterial` (`self.StaticMesh`) 0 _output_get)
  (`parent.ReceiveBeginPlay`))

(fn `AddWaterImpact`
  (params (ImpactLocation :type "Vector Structure") (ImpactStrength :type "Float (double-precision)"))
  (bind _watermid (`self.WaterMID`))
  (`/Engine/EditorBlueprintResources/StandardMacros.IsValid` _watermid
    (:`Is Valid`
      (`MaterialInstanceDynamic.SetVectorParameterValue` _watermid "RippleCenter" (`KismetMathLibrary.Conv_VectorToLinearColor` ImpactLocation))
      (`MaterialInstanceDynamic.SetScalarParameterValue` _watermid "RippleStartTime" (`KismetSystemLibrary.GetGameTimeInSeconds`))
      (`MaterialInstanceDynamic.SetScalarParameterValue` _watermid "RippleStrength" ImpactStrength))
    (:`Is Not Valid`
      (`KismetSystemLibrary.PrintString` "BP_EaterPlane_material not valid"))))

(fn `UserConstructionScript`
  (`parent.UserConstructionScript`)
  (bind _returnvalue (`KismetMaterialLibrary.CreateDynamicMaterialInstance` (`self.BaseMaterial`)))
  (bind _output_get (set `self.WaterMID` _returnvalue))
  (`PrimitiveComponent.SetMaterial` (`self.StaticMesh`) 0 _output_get))