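; BP_UnderwaterController is an underwater atmosphere controller that changes scene lighting as the player pawn descends below a surface height.
; Each tick it converts the player's depth below SurfaceZ, relative to MaxDepth, into a clamped 0–1 alpha.
; That alpha lerps height fog density and inscattering color, dims the directional light, and tints post-process gain toward blue by cutting red most.
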(event `self.ReceiveBeginPlay`
  (set `self.PlayerRef` (`GameplayStatics.GetPlayerPawn` 0)))

(event `self.ReceiveTick`
  (params (DeltaSeconds :type "Float (single-precision)"))
  (bind _postprocess (`self.PostProcess`))
  (bind _component (`ExponentialHeightFog.Component` (`self.FogRef`)))
  (bind _output_get (set `self.Depth01` (`KismetMathLibrary.FClamp` (/ (- (`self.SurfaceZ`) (.z (`self.K2_GetActorLocation` (`self.PlayerRef`)))) (`self.MaxDepth`)))))
  ; Fog
  (`ExponentialHeightFogComponent.SetFogDensity` _component (`KismetMathLibrary.Lerp` 0.02 0.06 _output_get))
  ; Directional Light
  (`LightComponent.SetIntensity` (`Light.LightComponent` (`self.DirLightRef`)) (`KismetMathLibrary.Lerp` 5.0 0.8 _output_get))
  ; Post Proccessing
  (bind _structout (setmembers `PostProcessSettings` :`StructRef` (`PostProcessComponent.Settings` _postprocess) :`ColorGain` (`KismetMathLibrary.MakeVector4` (`KismetMathLibrary.Lerp` 1.0 0.65 _output_get) (`KismetMathLibrary.Lerp` 1.0 0.8 _output_get) (`KismetMathLibrary.Lerp` 1.0 1.0 _output_get) 1.0)))
  (set `PostProcessComponent.Settings` _structout _postprocess)
  (`ExponentialHeightFogComponent.SetFogInscatteringColor` _component (`KismetMathLibrary.LinearColorLerp` (make `LinearColor` 0.05 0.18 0.3 1.0) (make `LinearColor` 0.01 0.05 0.1 1.0) _output_get)))

(fn `UserConstructionScript`)